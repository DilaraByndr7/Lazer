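; BP_Enemy is an enemy that repeatedly chases and damages the player.
; From BeginPlay, the Takip event runs AI MoveTo toward the player controller and calls itself again after each success or failure.
; Each successful move subtracts Damage from BP_ThirdPersonCharacter's HP and updates its health bar, passing zero as MaxHealth.
; ThirdPersonMap opens only when HP equals exactly zero, which ends the loop.
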(event `self.ReceiveBeginPlay`
  (`self.Takip`))

(event `Takip`
  (`|AIMoveTo` self (0.0 0.0 0.0) (`GameplayStatics.GetPlayerController` 0) 100.0
    (:`OnSuccess`
      (bind _returnvalue (`GameplayStatics.GetActorOfClass` "/Game/ThirdPerson/Blueprints/BP_ThirdPersonCharacter.BP_ThirdPersonCharacter_C"))
      (bind _output_get (set `/Game/ThirdPerson/Blueprints/BP_ThirdPersonCharacter.HP` (- (`/Game/ThirdPerson/Blueprints/BP_ThirdPersonCharacter.HP` _returnvalue) (`self.Damage`)) _returnvalue))
      (`/Game/UI/HealtBar_UI.UpdateHealth` (`/Game/ThirdPerson/Blueprints/BP_ThirdPersonCharacter.HBar_UI` _returnvalue) _output_get 0.0)
      (if (== _output_get 0.0)
        (`GameplayStatics.OpenLevel` "ThirdPersonMap")
        (else
          (`self.Takip`))))
    (:`OnFail`
      (`self.Takip`))))

(fn `UserConstructionScript`)